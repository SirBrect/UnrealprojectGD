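; BP_Doggo is a dog character that walks in a heading set by directional commands, with start and stop events.
; Each tick it repositions a TargetPoint just ahead along WalkDirection and uses navmesh move-to while moving.
; FaceDirection halts it and lerps its forward vector to the new heading, nudging rightward for exact reversals, then resumes walking.
; Forward matches the Human's facing, while Left, Right and Back are relative to the dog.
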(event `self.ReceiveTick`
  (params (DeltaSeconds :type "Float (single-precision)"))
  ;[1 1 1] Tick
  (if (`self.moving`)
    (`AIBlueprintHelperLibrary.SimpleMoveToLocation` (`self.GetController`) (`self.K2_GetActorLocation` (`self.targetPoint`))))
  (if (<= 0.1 (`self.GetDistanceTo` (`self.targetPoint`)))
    (`self.K2_SetActorTransform` (`self.targetPoint`) (`KismetMathLibrary.Conv_VectorToTransform` (+ (* (`self.walkDirection`) 10.0) (`self.K2_GetActorLocation`))) false false))
  (if (`self.rotating`)
    (if (== (`self.GetActorForwardVector`) (`KismetMathLibrary.NegateVector` (`self.targetRotationVector`)))
      (`self.K2_SetActorRotation` (`KismetMathLibrary.Conv_VectorToRotator` (`KismetMathLibrary.VLerp` (`self.GetActorForwardVector`) (`self.GetActorRightVector`) 0.03))))
    (`self.K2_SetActorRotation` (`KismetMathLibrary.Conv_VectorToRotator` (`KismetMathLibrary.VLerp` (`self.GetActorForwardVector`) (`self.targetRotationVector`) (`self.myAlpha`))))
    (set `self.myAlpha` (+ (`self.myAlpha`) (* (`self.rotateSpeed`) (`GameplayStatics.GetWorldDeltaSeconds`))))
    (if (== (`self.GetActorForwardVector`) (`self.targetRotationVector`))
      (set `self.rotating` false)
      (set `self.moving` true)
      (set `self.walkDirection` (`self.GetActorForwardVector`)))))

(event `Face Direction`
  (params (Direction :type String))
  ;[1 1 1] Face Direction
  (set `self.walkDirection` (0.0 0.0 0.0))
  (set `self.moving` false)
  (set `self.myAlpha` 0.0)
  (switch `string` Direction
    (:`Forward`
      (set `self.targetRotationVector` (`self.GetActorForwardVector` (`self.human`))))
    (:`Left`
      (set `self.targetRotationVector` (`KismetMathLibrary.NegateVector` (`self.GetActorRightVector`))))
    (:`Right`
      (set `self.targetRotationVector` (`self.GetActorRightVector`)))
    (:`Back`
      (set `self.targetRotationVector` (`KismetMathLibrary.NegateVector` (`self.GetActorForwardVector`)))))
  (set `self.rotating` true))

(event `startMoving`
  ;[1 1 1] Start/Stop
  (set `self.moving` true))

(event `stopMoving`
  ;[1 1 1] Start/Stop
  (set `self.moving` false))

(fn `GetMoving`
  (returns (`isMoving?` :type Boolean))
  (return (`self.moving`)))

(fn `UserConstructionScript`)